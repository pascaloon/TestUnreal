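; Moving platform actor that travels back and forth between two points marked by its Sphere1 and Sphere2 components.
; BeginPlay caches both spheres' world locations as fixed endpoints.
; Tick lerps the actor between them without sweep, using Abs(Sin(Progress)) as alpha, and adds Speed to Progress each frame, so movement is frame-rate dependent.
; An older linear ping-pong using a State flag remains unconnected.
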(event `self.ReceiveBeginPlay`
  (set `self.Position1` (`SceneComponent.K2_GetComponentLocation` (`self.Sphere1`)))
  (set `self.Position2` (`SceneComponent.K2_GetComponentLocation` (`self.Sphere2`))))

(event `self.ReceiveTick`
  (params (DeltaSeconds :type "Float (single-precision)"))
  (`self.K2_SetActorLocation` (`KismetMathLibrary.VLerp` (`self.Position1`) (`self.Position2`) (`KismetMathLibrary.Abs` (`KismetMathLibrary.Sin` (`self.Progress`)))))
  (set `self.Progress` (+ (`self.Progress`) (`self.Speed`))))

(event `self.ReceiveBeginPlay`)

(event `self.ReceiveActorBeginOverlap`
  (params (OtherActor :type "Actor Object Reference")))

(fn `UserConstructionScript`)